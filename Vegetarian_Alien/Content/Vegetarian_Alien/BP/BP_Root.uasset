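; BP_Root is a short-lived actor, apparently a root pickup, that flies to the player when it spawns.
; On BeginPlay it spawns an NS_Poof effect at its XY position and a fixed height, then starts PickUpTimeline.
; Each update lerps from its current location toward player pawn 0's live position, so the motion compounds and homes in.
; The actor destroys itself when the timeline finishes.
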(event EventBeginPlay
  (bind _returnvalue (Transformation|GetActorLocation))
  (bind (_x _y) (Math|Vector|BreakVector _returnvalue))
  (Niagara|SpawnSystematLocation "/Game/Vegetarian_Alien/FX/VFX/NS_Poof.NS_Poof" (Math|Vector|MakeVector _x _y 6e+01))
  (bind _pickuptrack (Timeline|PickUpTimeline PlayFromStart)
    (:Update
      (Transformation|SetActorLocation (Math|Vector|Lerp(Vector) (Transformation|GetActorLocation) (Transformation|GetActorLocation (Game|Player|GetPlayerPawn 0)) _pickuptrack) false false))
    (:Finished
      (Actor|DestroyActor))))

(fn ConstructionScript)