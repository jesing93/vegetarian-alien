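; Main menu controller that turns tagged static meshes in the level into clickable 3D Play, Tutorial and Exit buttons.
; On BeginPlay it adds the Menu widget, resets the game instance's level counter and gathers MenuButton-tagged meshes.
; Mouse traces every tick swap matching buttons to emissive materials with a hover sound.
; Clicks read the second component tag to open Level_Final, show the tutorial or quit.
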(event Custom|ClearMenuButtons
  (if (Variables|Default|GetButtonHovered)
    (for _array_element (Variables|Default|GetMenuButtons)
      (if (Components|ComponentHasTag (Actor|GetComponentbyClass _array_element "/Script/Engine.StaticMeshComponent") "YellowButton")
        (Rendering|Material|SetMaterial (Actor|GetComponentbyClass _array_element "/Script/Engine.StaticMeshComponent") 0 "/Game/Vegetarian_Alien/2D/M_ButtonInside.M_ButtonInside")
        (else
          (Rendering|Material|SetMaterial (Actor|GetComponentbyClass _array_element "/Script/Engine.StaticMeshComponent") 0 "/Game/Vegetarian_Alien/2D/M_ButtonOutside.M_ButtonOutside"))))
    (Variables|Default|SetButtonHovered false)))

(event EventBeginPlay
  (bind _returnvalue (UserInterface|CreateWidget "/Game/Vegetarian_Alien/Widget/Menu.Menu_C"))
  (bind _output_get (Variables|Default|SetMenuUI _returnvalue))
  (UserInterface|Viewport|AddtoViewport _output_get 0)
  (Variables|/Script/Engine.PlayerController|SetbShowMouseCursor (Game|GetPlayerController 0) true)
  (Variables|/Game/Vegetarian_Alien/BP/BP_GameInstance.BP_GameInstance_C|SetActualLevel (.AsBP%20Game%20Instance (Utilities|Casting|CastToBP_GameInstance (Game|GetGameInstance))) 0)
  (Input|SetInputModeGameandUI (Game|GetPlayerController 0) (Variables|Default|GetMenuUI) "DoNotLock" true false)
  (bind _outactors (Actor|GetAllActorsOfClass "/Script/Engine.StaticMeshActor"))
  (for _array_element _outactors
    (if (Components|ComponentHasTag (Actor|GetComponentbyClass _array_element "/Script/Engine.StaticMeshComponent") "MenuButton")
      (Utilities|Array|Add (Variables|Default|GetMenuButtons) _array_element))))

(event EventTick
  (params (DeltaSeconds :type Float%20%28single-precision%29))
  (bind _returnvalue (Game|GetPlayerController 0))
  (bind (_worldlocation _worlddirection) (Game|Player|ConvertMouseLocationToWorldSpace _returnvalue))
  (bind (_outhit _returnvalue_2) (Collision|LineTraceByChannel _worldlocation (+ _worldlocation (* _worlddirection 1e+04)) "TraceTypeQuery1" false 0 "None"))
  (if _returnvalue_2
    (Utilities|IsValid (Actor|GetComponentbyClass (.HitActor (Collision|BreakHitResult _outhit)) "/Script/Engine.StaticMeshComponent")
      (:Is%20Valid
        (if (Components|ComponentHasTag (Actor|GetComponentbyClass (.HitActor (Collision|BreakHitResult _outhit)) "/Script/Engine.StaticMeshComponent") "MenuButton")
          (if (not (Variables|Default|GetButtonHovered))
            (for _array_element (Variables|Default|GetMenuButtons)
              (if (== (Utilities|Array|Get(acopy) (Variables|/Script/Engine.ActorComponent|GetComponentTags (Actor|GetComponentbyClass (.HitActor (Collision|BreakHitResult _outhit)) "/Script/Engine.StaticMeshComponent")) 1) (Utilities|Array|Get(acopy) (Variables|/Script/Engine.ActorComponent|GetComponentTags (Actor|GetComponentbyClass _array_element "/Script/Engine.StaticMeshComponent")) 1))
                (if (Components|ComponentHasTag (Actor|GetComponentbyClass _array_element "/Script/Engine.StaticMeshComponent") "YellowButton")
                  (Rendering|Material|SetMaterial (Actor|GetComponentbyClass _array_element "/Script/Engine.StaticMeshComponent") 0 "/Game/Vegetarian_Alien/2D/M_ButtonInside_Emissive.M_ButtonInside_Emissive")
                  (else
                    (Rendering|Material|SetMaterial (Actor|GetComponentbyClass _array_element "/Script/Engine.StaticMeshComponent") 0 "/Game/Vegetarian_Alien/2D/M_ButtonOutside_Emissive.M_ButtonOutside_Emissive")))
                (Variables|Default|SetButtonHovered true)
                (Audio|PlaySound2D "/Game/Vegetarian_Alien/FX/Sounds/S_ButtonHover.S_ButtonHover" 1.0 1.0 0.0 0 0))))
          (else
            (CallFunction|ClearMenuButtons :!label _label))))
      (:Is%20Not%20Valid
        (goto _label)))
    (else
      (goto _label))))

(event Input|MouseEvents|LeftMouseButton
  (params (Key :type Key%20Structure :default "None"))
  (bind _returnvalue (Game|GetPlayerController 0))
  (bind (_worldlocation _worlddirection) (Game|Player|ConvertMouseLocationToWorldSpace _returnvalue))
  (:Pressed
    (bind (_outhit _returnvalue_2) (Collision|LineTraceByChannel _worldlocation (+ _worldlocation (* _worlddirection 1e+04)) "TraceTypeQuery1" false 0 "None"))
    (if _returnvalue_2
      (Utilities|IsValid (Actor|GetComponentbyClass (.HitActor (Collision|BreakHitResult _outhit)) "/Script/Engine.StaticMeshComponent")
        (:Is%20Valid
          (if (Components|ComponentHasTag (Actor|GetComponentbyClass (.HitActor (Collision|BreakHitResult _outhit)) "/Script/Engine.StaticMeshComponent") "MenuButton")
            (switch name (Utilities|Array|Get(acopy) (Variables|/Script/Engine.ActorComponent|GetComponentTags (Actor|GetComponentbyClass (.HitActor (Collision|BreakHitResult _outhit)) "/Script/Engine.StaticMeshComponent")) 1)
              (:PlayButton
                (Game|OpenLevel(byObjectReference) "/Game/Vegetarian_Alien/Maps/Level_Final.Level_Final"))
              (:TutorialButton
                (Input|SetInputModeUIOnly (Game|GetPlayerController 0) (Variables|Default|GetMenuUI) "DoNotLock" false)
                (Default|ShowTutorial (Variables|Default|GetMenuUI)))
              (:ExitButton
                (Game|QuitGame 0 "Quit" false)))))))))

(fn ConstructionScript)