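; BP_Farmer is an NPC farmer that roams the level and chases the player, the plant, when told to follow.
; Tick uses SimpleMoveToLocation toward either the player's ground position or a random reachable navmesh point, which NewLocation replaces once the farmer gets close.
; Follow and Unfollow events switch between chasing and roaming, raising walk speed for the chase and restoring it afterward.
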(event Custom|Follow
  ;[1 1 1] Going to catch the plant
  (Variables|Default|SetFollowing true)
  (Variables|/Script/Engine.CharacterMovementComponent|SetMaxWalkSpeed (Variables|Character|GetCharacterMovement) 4e+02))

(event Custom|Unfollow
  ;[1 1 1] Stop going to catch the plant
  (Variables|Default|SetFollowing false)
  (CallFunction|NewLocation)
  (Variables|/Script/Engine.CharacterMovementComponent|SetMaxWalkSpeed (Variables|Character|GetCharacterMovement) 2e+02))

(event Custom|NewLocation
  ;[1 1 1] New reachable location generator
  (Variables|Default|SetTargetLocation (.RandomLocation (AI|Navigation|GetRandomReachablePointinRadius (Transformation|GetActorLocation) 2.5e+03 0 0))))

(event EventTick
  (params (DeltaSeconds :type Float%20%28single-precision%29))
  (bind _returnvalue (Transformation|GetActorLocation))
  (bind _returnvalue_2 (Game|Player|GetPlayerPawn 0))
  (bind _targetlocation (Variables|Default|GetTargetLocation))
  (bind (_x _y) (Math|Vector|BreakVector _returnvalue))
  (bind _returnvalue_3 (Transformation|GetActorLocation _returnvalue_2))
  (bind (_x_2 _y_2) (Class|KismetMathLibrary|BreakVector3f _returnvalue_3))
  ;[1 1 1] Movement
  (if (Variables|Default|GetFollowing)
    ;;[1 1 1] Following movement
    (AI|Navigation|SimpleMovetoLocation (Pawn|GetController) (Math|Vector|MakeVector _x_2 _y_2 0.0))
    (elif (Utilities|Operators|EqualEqual _targetlocation (Math|Vector|MakeVector _x _y 1e+01) 1e+02)
      ;;[1 1 1] Set new location when reaching
      (CallFunction|NewLocation)
      (else
        ;;[1 1 1] Random movement
        (AI|Navigation|SimpleMovetoLocation (Pawn|GetController) _targetlocation)))))

(event EventBeginPlay
  ;[1 1 1] Set initial random roam location
  (CallFunction|NewLocation))

(fn ConstructionScript)